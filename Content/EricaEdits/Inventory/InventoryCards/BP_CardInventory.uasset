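; BP_CardInventory is a card pickup actor for the inventory that plays narration when picked up.
; BeginPlay applies the configured material to its Cube.
; PickUpItem prints a debug string, calls ItemPickUpSounds and returns Item and ItemObj.
; ItemPickUpSounds uses the CardOverlap flag to block repeat narration until the clip's duration elapses; the pickup sound, end sound and DestroyActor nodes are disconnected, so the actor never destroys itself.
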(event `self.ReceiveBeginPlay`
  (`PrimitiveComponent.SetMaterial` (`self.Cube`) 0 (`self.Material`)))

(event `self.ReceiveActorEndOverlap`
  (params (OtherActor :type "Actor Object Reference")))

(event `ItemPickUpSounds`
  (bind _narration (`self.Narration`))
  ;[1 1 1] Prevents sound repeat and plays narration, deletes after playing
  (if (`self.CardOverlap`)
    (set `self.CardOverlap` false)
    (`GameplayStatics.PlaySoundAtLocation` _narration (`self.K2_GetActorLocation`) (struct) 1.0 1.0 0.0 null null null null)
    (`KismetSystemLibrary.Delay` (`SoundBase.Duration` _narration))
    (set `self.CardOverlap` true)))

(fn `PickUpItem`
  (returns (Item :type String) (ItemObj :type "Actor Object Reference"))
  (`KismetSystemLibrary.PrintString` "Item up")
  (`self.ItemPickUpSounds`)
  (return (`self.Item`) (`self.ItemObj`)))

(fn `UserConstructionScript`)