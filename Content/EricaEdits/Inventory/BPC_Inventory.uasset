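; BPC_Inventory is an inventory component that records picked items and their objects in two arrays.
; AddItemToInventory appends to Inventory and InventoryObject, printing debug messages as it goes.
; It then copies each array to BP_BookInventory02's list variables, but only if the same owner casts to both ThrusterVRCharater and BP_BookInventory02.
; The character's PlayInventoryCardMessage call is disconnected and never runs.
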(fn `AddItemToInventory`
  (params (NewItem :type "String (by ref)") (NewInvObj :type "Actor Object Reference"))
  (bind _returnvalue (`self.GetOwner`))
  (bind _returnvalue_2 (`self.GetOwner`))
  (`|ExecutionSequence`
    (:`then_0`
      (`KismetArrayLibrary.Array_Add` (`self.Inventory`) NewItem)
      (`KismetSystemLibrary.PrintString` NewItem)
      (bind _asthruster_vrcharater (cast `/Game/EricaEdits/Blueprints/ThrusterVRCharater` _returnvalue_2))
      (bind _asbp_book_inventory_02 (cast `/Game/EricaEdits/Blueprints/BP_BookInventory02` _returnvalue_2))
      (set `/Game/EricaEdits/Blueprints/BP_BookInventory02.ListItem` (`self.Inventory`) _asbp_book_inventory_02))
    (:`then_1`
      (`KismetArrayLibrary.Array_Add` (`self.InventoryObject`) NewInvObj)
      (`KismetSystemLibrary.PrintString` "Oh look new object")
      (cast `/Game/EricaEdits/Blueprints/ThrusterVRCharater` _returnvalue)
      (bind _asbp_book_inventory_02_2 (cast `/Game/EricaEdits/Blueprints/BP_BookInventory02` _returnvalue))
      (set `/Game/EricaEdits/Blueprints/BP_BookInventory02.ListItemObj` (`self.InventoryObject`) _asbp_book_inventory_02_2))))