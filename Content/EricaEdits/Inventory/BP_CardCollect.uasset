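; BP_CardCollect is a collectible card item that plays narration when picked up and then removes itself.
; PickUpItem prints a debug string, triggers ItemPickUpSounds and returns the card's Item and ItemObj to the caller.
; ItemPickUpSounds clears the CardOverlap flag to block repeats, then plays pickup, narration and end sounds at the actor's location, chained by duration-based delays before DestroyActor.
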(event `self.ReceiveActorEndOverlap`
  (params (OtherActor :type "Actor Object Reference")))

(event `ItemPickUpSounds`
  (bind _returnvalue (`self.K2_GetActorLocation`))
  (bind _narration (`self.Narration`))
  (bind _pickupsound (`self.PickupSound`))
  (bind _end_sound (`self.End Sound`))
  ;[1 1 1] Prevents sound repeat and plays narration, deletes after playing
  (if (`self.CardOverlap`)
    (set `self.CardOverlap` false)
    (`GameplayStatics.PlaySoundAtLocation` _pickupsound _returnvalue (struct) 1.0 1.0 0.0 null null null null)
    (`KismetSystemLibrary.Delay` (`SoundBase.Duration` _pickupsound))
    (`GameplayStatics.PlaySoundAtLocation` _narration _returnvalue (struct) 1.0 1.0 0.0 null null null null)
    (`KismetSystemLibrary.Delay` (`SoundBase.Duration` _narration))
    (`GameplayStatics.PlaySoundAtLocation` _end_sound _returnvalue (struct) 1.0 1.0 0.0 null null null null)
    (`KismetSystemLibrary.Delay` (`SoundBase.Duration` _end_sound))
    (`self.K2_DestroyActor`)))

(fn `PickUpItem`
  (returns (Item :type String) (ItemObj :type "Actor Object Reference"))
  (`KismetSystemLibrary.PrintString` "Item up")
  (`self.ItemPickUpSounds`)
  (return (`self.Item`) (`self.ItemObj`)))

(fn `UserConstructionScript`)