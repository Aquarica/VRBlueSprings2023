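; BP_BookInventory02 is a Blueprint for a book-style inventory that shows collected cards.
; PlayInventoryCard stores the passed item array in ListItem and makes the Card01 and Card02 components visible when their names are present.
; Cards are only ever revealed, never hidden; FillInventory and PickUpItem are empty stubs, and BeginPlay just prints a debug message.
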(event `FillInventory`
  (params (NewParam :type Boolean)))

(event `self.ReceiveBeginPlay`
  (`KismetSystemLibrary.PrintString` "Hello inventoryu"))

(event `self.ReceiveTick`
  (params (DeltaSeconds :type "Float (single-precision)")))

(event `/Game/EricaEdits/Inventory/BPI_Pickup.PlayInventoryCard`
  (params (InventoryArray :type "Array of String (by ref)"))
  (set `self.ListItem` InventoryArray)
  (`|ExecutionSequence`
    (:`then_0`
      (if (`KismetArrayLibrary.Array_Contains` (`self.ListItem`) "Card01")
        (`SceneComponent.SetVisibility` (`self.Card01`) true false)))
    (:`then_1`
      (if (`KismetArrayLibrary.Array_Contains` (`self.ListItem`) "Card02")
        (`SceneComponent.SetVisibility` (`self.Card02`) true false)))))

(fn `PickUpItem`
  (returns (Item :type String) (ItemObj :type "Actor Object Reference"))
  (return "" null))

(fn `UserConstructionScript`)